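; Mordhau build-box equipment that lets players cycle through deployables and place them, spending ammo per object.
; Each tick BuildingSystem validates and previews the spot, adding rules for Frontline-only deployable spawns, while the HUD shows placed counts and failure reasons.
; Firing sends a transform relative to the hit component to the server, which rechecks range and cost, spawns, optionally attaches (never to landscape), and retires objects displaced by per-player limits.
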(event `self.LocalPlayerLateTick`
  (params (DeltaTime :type "Float (single-precision)"))
  (bind _buildingsystem (`self.BuildingSystem`))
  (`|ExecutionSequence`
    (:`then_0`
      ;[1 1 1] Hacky way to prevent deploy spawns showing in other modes
      (cast `/Game/Mordhau/Blueprints/GameModes/Battle/BP_FrontlineGameState` (`GameplayStatics.GetGameState`)
        (:`CastFailed`
          (if (== (`.ActorClass` (break `SpawnableObjectInfo` (`|GetArrayItem` (`BuildingSystemComponent.SpawnableObjects` (`self.BuildingSystem`)) (`self.ObjectType`)))) "/Game/Mordhau/Blueprints/Interactables/Environment/Specific/BP_DeployableSpawn.BP_DeployableSpawn_C")
            (`BuildingSystemComponent.DestroyMeshPreview` _buildingsystem)
            (`self.CycleObjectType`)))))
    (:`then_1`
      (bind _returnvalue (`BuildingSystemComponent.GetEquipmentAmmoCost` (`self.BuildingSystem`) (`self.ObjectType`)))
      (bind _returnvalue_2 (< (`self.GetAmmo`) (`KismetMathLibrary.Conv_IntToByte` _returnvalue)))
      (if (or (<= (`GameplayStatics.GetTimeSeconds`) (`self.NextAvailableTime`)) _returnvalue_2)
        (`BuildingSystemComponent.DestroyMeshPreview` _buildingsystem)
        (if _returnvalue_2
          (`self.CycleObjectType`))
        (else
          (`self.ValidateSpotWithBuildingSystem` (0.0 0.0 0.0) true))))))

(event `self.UpdateEquipmentState`
  (`parent.UpdateEquipmentState`)
  (`BuildingSystemComponent.DestroyMeshPreview` (`self.BuildingSystem`)))

(event `self.OnDropped`
  (params (Character :type "MordhauCharacter Object Reference"))
  (`parent.OnDropped` Character)
  (`self.K2_DestroyActor`))

(event `ServerRequestPlant`
  (params (Location :type "Vector Structure") (Rotation :type "Rotator Structure") (ObjectType :type Byte) (AttachTo :type "SceneComponent Object Reference"))
  (`self.RequestPlant` Location Rotation ObjectType AttachTo))

(event `self.BuildingSystem.OnMeshPreviewCreated`
  (`self.OnShowWidget`)
  (`self.UpdateEquipmentUI`))

(event `self.BuildingSystem.OnMeshPreviewDestroyed`
  (`self.OnHideWidget`))

(event `self.K2_OnBecomeViewTarget`
  (params (PC :type "PlayerController Object Reference"))
  (`parent.K2_OnBecomeViewTarget` PC)
  (if (== (`Controller.GetViewTarget` PC) (`self.GetOwner`))
    (`self.OnShowWidget`)))

(event `OnBindEventToPlaceablesUpdate`
  (bind _returnvalue (`self.GetParentCharacter`))
  (`/Engine/EditorBlueprintResources/StandardMacros.IsValid` _returnvalue
    (:`Is Valid`
      (bind _asbp_mordhau_player_controller (cast `/Game/Mordhau/Blueprints/BP_MordhauPlayerController` (`Pawn.GetController` _returnvalue)))
      (add `/Game/Mordhau/Blueprints/BP_MordhauPlayerController.EventOnPlaceablesUpdate` _asbp_mordhau_player_controller (delegate `EventOnPlaceablesUpdate`)))))

(event `EventOnPlaceablesUpdate`
  (`self.UpdateEquipmentUI`))

(event `OnUnbindEventToPlaceablesUpdate`
  (bind _returnvalue (`self.GetParentCharacter`))
  (`/Engine/EditorBlueprintResources/StandardMacros.IsValid` _returnvalue
    (:`Is Valid`
      (bind _asbp_mordhau_player_controller (cast `/Game/Mordhau/Blueprints/BP_MordhauPlayerController` (`Pawn.GetController` _returnvalue)))
      (remove `/Game/Mordhau/Blueprints/BP_MordhauPlayerController.EventOnPlaceablesUpdate` _asbp_mordhau_player_controller (delegate `EventOnPlaceablesUpdate`)))))

(fn `AddSkeletalMeshPreviewIfNone`
  (params (SkeletalMesh :type "SkeletalMesh Object Reference"))
  (bind _asskeletal_mesh_component (cast `SkeletalMeshComponent` (`self.PreviewMeshComponent`))
    (:`then`
      (if (!= (`SkinnedMeshComponent.SkeletalMesh` _asskeletal_mesh_component) SkeletalMesh)
        (`self.DestroyMeshPreview` :!label _label)
        (bind _returnvalue (`AddComponent|NODE_AddSkeletalMeshComponent-0`))
        (`SkinnedMeshComponent.SetSkinnedAssetAndUpdate` _returnvalue SkeletalMesh true)
        (set `self.PreviewMeshComponent` _returnvalue)
        (`self.SetupMeshPreview`)))
    (:`CastFailed`
      (goto _label))))

(fn `AddStaticMeshPreviewIfNone`
  (params (StaticMesh :type "StaticMesh Object Reference"))
  (bind _asstatic_mesh_component (cast `StaticMeshComponent` (`self.PreviewMeshComponent`))
    (:`then`
      (if (!= (`StaticMeshComponent.StaticMesh` _asstatic_mesh_component) StaticMesh)
        (`self.DestroyMeshPreview` :!label _label)
        (bind _returnvalue (`AddComponent|NODE_AddStaticMeshComponent-1`))
        (`StaticMeshComponent.SetStaticMesh` _returnvalue StaticMesh)
        (set `self.PreviewMeshComponent` _returnvalue)
        (`self.SetupMeshPreview`)))
    (:`CastFailed`
      (goto _label))))

(fn `CycleObjectType`
  (bind _spawnableobjects (`BuildingSystemComponent.SpawnableObjects` (`self.BuildingSystem`)))
  (bind _returnvalue (- (`KismetArrayLibrary.Array_Length` _spawnableobjects) 0))
  (for _index (range 1 (+ _returnvalue 1))
    (bind _returnvalue_2 (mod (+ (`self.ObjectType`) _index) _returnvalue))
    (if (<= (`.Cost` (break `SpawnableObjectInfo` (`|GetArrayItem` _spawnableobjects _returnvalue_2))) (`self.GetAmmo`))
      (set `self.ObjectType` _returnvalue_2)
      (`self.UpdateEquipmentUI`)
      (break))))

(fn `DestroyMeshPreview`
  (bind _previewmeshcomponent (`self.PreviewMeshComponent`))
  (bind _widgetdisplay (`self.WidgetDisplay`))
  (`|ExecutionSequence`
    (:`then_0`
      (`/Engine/EditorBlueprintResources/StandardMacros.IsValid` _widgetdisplay
        (:`Is Valid`
          (`ActorComponent.K2_DestroyComponent` _widgetdisplay)
          (set `self.WidgetDisplay` null))))
    (:`then_1`
      (`/Engine/EditorBlueprintResources/StandardMacros.IsValid` _previewmeshcomponent
        (:`Is Valid`
          (`ActorComponent.K2_DestroyComponent` _previewmeshcomponent)
          (set `self.PreviewMeshComponent` null))))))

(fn `GetAmountOfPlacedEquipment`
  (params (PlaceableEquipmentName :type Name))
  (returns (Amount :type Integer))
  (bind _returnvalue (`self.GetParentCharacter`))
  (if (`KismetSystemLibrary.IsValid` _returnvalue)
    (bind _asbp_mordhau_player_controller (cast `/Game/Mordhau/Blueprints/BP_MordhauPlayerController` (`Pawn.GetController` _returnvalue)))
    (bind (_value _returnvalue_2) (`BlueprintMapLibrary.Map_Find` (`/Game/Mordhau/Blueprints/BP_MordhauPlayerController.PlaceablesMap` _asbp_mordhau_player_controller) PlaceableEquipmentName))
    (if _returnvalue_2
      (return (`KismetMathLibrary.Conv_ByteToInt` _value))
      (else
        (return 0)))))

(fn `OnHideWidget`
  (`MordhauHUDWidgetComponent.HideWidget` (`self.MordhauHUDWidget`))
  (`self.OnUnbindEventToPlaceablesUpdate`))

(fn `OnRequestFire`
  (params (Character :type "MordhauCharacter Object Reference"))
  (returns (ReturnValue :type Boolean))
  (bind _returnvalue (`GameplayStatics.GetTimeSeconds`))
  (bind _objecttype (`self.ObjectType`))
  (bind _spawnableobjects (`BuildingSystemComponent.SpawnableObjects` (`self.BuildingSystem`)))
  (bind (_preview _previewskeletal _cost _rotationoffset _rotationoffsetpreview _nothitrotationpreviewoffset _nothitlocationpreviewoffset _scalepreview _actorclass _displayname _placablelimitname _placeablelimitmax _spawnactoroffset) (break `SpawnableObjectInfo` (`|GetArrayItem` _spawnableobjects _objecttype)))
  (`/Engine/EditorBlueprintResources/StandardMacros.IsValid` Character
    (:`Is Valid`
      (set `MordhauCharacter.bWantsFire` false Character))
    (:`Is Not Valid`
      _))
  (if (`KismetArrayLibrary.Array_IsValidIndex` _spawnableobjects _objecttype)
    (if (and (> _returnvalue (`self.NextAvailableTime`)) (>= (`self.GetAmmo`) _cost))
      (bind (_succeeded _location _rotation _attachtocomponent) (`self.ValidateSpotWithBuildingSystem` (0.0 0.0 0.0)))
      (if _succeeded
        (set `self.NextAvailableTime` (+ _returnvalue (`self.Cooldown`)))
        (bind _returnvalue_2 (`SceneComponent.K2_GetComponentToWorld` _attachtocomponent))
        (bind _returnvalue_3 (`KismetMathLibrary.ComposeRotators` _rotationoffset _rotation))
        (`self.ServerRequestPlant` (`KismetMathLibrary.InverseTransformLocation` _returnvalue_2 (+ _location (`KismetMathLibrary.GreaterGreater_VectorRotator` _spawnactoroffset _returnvalue_3))) (`KismetMathLibrary.InverseTransformRotation` _returnvalue_2 _returnvalue_3) (`KismetMathLibrary.Conv_IntToByte` (`self.ObjectType`)) _attachtocomponent)))
    (return false)))

(fn `OnRequestModeSwitch`
  (params (Character :type "MordhauCharacter Object Reference"))
  (returns (ReturnValue :type Boolean))
  (`self.CycleObjectType`)
  (return true))

(fn `OnShowWidget`
  (`MordhauHUDWidgetComponent.ShowWidget` (`self.MordhauHUDWidget`))
  (`self.Update Trace Text` "" true)
  (`self.OnBindEventToPlaceablesUpdate`))

(fn `RequestPlant`
  (params (Location :type "Vector Structure") (Rotation :type "Rotator Structure") (ObjectType :type Byte) (AttachTo :type "SceneComponent Object Reference"))
  (locals (WantsAttach :type Boolean))
  (bind _returnvalue (`self.GetParentCharacter`))
  (bind _returnvalue_2 (`SceneComponent.K2_GetComponentToWorld` AttachTo))
  (bind _returnvalue_3 (`ActorComponent.GetOwner` AttachTo))
  (bind _returnvalue_4 (`KismetMathLibrary.Conv_ByteToInt` ObjectType))
  (bind _returnvalue_5 (`KismetMathLibrary.TransformLocation` _returnvalue_2 Location))
  (bind _returnvalue_6 (`KismetMathLibrary.Conv_ByteToInt` (`self.GetAmmo`)))
  (bind _spawnableobjects (`BuildingSystemComponent.SpawnableObjects` (`self.BuildingSystem`)))
  (bind (_preview _previewskeletal _cost _rotationoffset _rotationoffsetpreview _nothitrotationpreviewoffset _nothitlocationpreviewoffset _scalepreview _actorclass _displayname _placablelimitname _placeablelimitmax _spawnactoroffset _bdonotattach) (break `SpawnableObjectInfo` (`|GetArrayItem` _spawnableobjects _returnvalue_4)))
  (bind _returnvalue_7 (`KismetMathLibrary.Conv_ByteToInt` _cost))
  (`/Engine/EditorBlueprintResources/StandardMacros.IsValid` AttachTo
    (:`Is Valid`
      (`/Engine/EditorBlueprintResources/StandardMacros.IsValid` _returnvalue
        (:`Is Valid`
          (bind _asbp_mordhau_player_controller (cast `/Game/Mordhau/Blueprints/BP_MordhauPlayerController` (`Pawn.GetController` _returnvalue)))
          (if (== _returnvalue_5 (`self.K2_GetActorLocation` _returnvalue) :`ErrorTolerance` 500.0)
            (if (`KismetArrayLibrary.Array_IsValidIndex` _spawnableobjects _returnvalue_4)
              (if (>= _returnvalue_6 _returnvalue_7)
                (if (and (not (`.bSuccess` (cast `MordhauEquipment` _returnvalue_3 :!pure true))) (not (`.bSuccess` (cast `Pawn` _returnvalue_3 :!pure true))) (not (`.bSuccess` (cast `MordhauProjectile` _returnvalue_3 :!pure true))))
                  (bind _returnvalue_8 (`|SpawnActorFromClass` _actorclass (`KismetMathLibrary.MakeTransform` _returnvalue_5 (`KismetMathLibrary.TransformRotation` _returnvalue_2 Rotation)) "Undefined" "OverrideRootScale" _asbp_mordhau_player_controller null))
                  (`|ExecutionSequence`
                    (:`then_0`
                      (`/Game/Mordhau/Blueprints/BP_MordhauPlayerController.OnBuilt` _asbp_mordhau_player_controller _returnvalue_8)
                      (`/Engine/EditorBlueprintResources/StandardMacros.IsValid` _returnvalue_8
                        (:`Is Valid`
                          (cast `LandscapeHeightfieldCollisionComponent` AttachTo
                            (:`then`
                              _)
                            (:`CastFailed`
                              (cast `LandscapeMeshCollisionComponent` AttachTo ; Landscape scale is too extreme and replication can't hnadle due to compression
                                (:`then`
                                  _)
                                (:`CastFailed`
                                  (set `local.WantsAttach` (not _bdonotattach))))))
                          (`|ExecutionSequence`
                            (:`then_0`
                              (bind _asmordhau_player_state (cast `MordhauPlayerState` (`Controller.PlayerState` _asbp_mordhau_player_controller)))
                              (`AddComponent|NODE_AddBP_BuildableComponent-1` :`self` _returnvalue_8 :`Builder` _asmordhau_player_state :`PlaceableLimitName` _placablelimitname :`OrignPlanterController` _asbp_mordhau_player_controller)
                              (bind _asbp_destroyable_deploy_spike_wall (cast `/Game/Mordhau/Blueprints/Interactables/Environment/Specific/BP_DestroyableDeploySpikeWall` _returnvalue_8))
                              (set `/Game/Mordhau/Blueprints/Interactables/Environment/Specific/BP_DestroyableDeploySpikeWall.PlanterController` _asbp_mordhau_player_controller _asbp_destroyable_deploy_spike_wall))
                            (:`then_1`
                              (if (`local.WantsAttach`)
                                (`self.K2_AttachToComponent` _returnvalue_8 AttachTo "None" "KeepWorld" "KeepWorld" "KeepWorld" false)))
                            (:`then_2`
                              (`self.SetAmmo` (`KismetMathLibrary.Conv_IntToByte` (- _returnvalue_6 _returnvalue_7)))
                              (bind _removedactor (`/Game/Mordhau/Blueprints/BP_MordhauPlayerController.PlaceInPlaceableArray` _asbp_mordhau_player_controller _placablelimitname _returnvalue_8 _placeablelimitmax))
                              (`/Engine/EditorBlueprintResources/StandardMacros.IsValid` _removedactor
                                (:`Is Valid`
                                  (`|ExecutionSequence`
                                    (:`then_0`
                                      (bind _returnvalue_9 (`self.GetComponentByClass` _removedactor "/Game/Mordhau/Blueprints/Interactables/BP_BuildableComponent.BP_BuildableComponent_C"))
                                      (if (`KismetSystemLibrary.IsValid` _returnvalue_9)
                                        (set `/Game/Mordhau/Blueprints/Interactables/BP_BuildableComponent.HasNotifiedDestruction` true _returnvalue_9)))
                                    (:`then_1`
                                      (bind _asbp_destroyable_actor (cast `/Game/Mordhau/Blueprints/Interactables/Environment/BP_DestroyableActor` _removedactor)
                                        (:`then`
                                          (`/Game/Mordhau/Blueprints/Interactables/Environment/BP_DestroyableActor.SetHealth` _asbp_destroyable_actor 0.0 null))
                                        (:`CastFailed`
                                          (bind _asadvanced_character (cast `AdvancedCharacter` _removedactor)
                                            (:`then`
                                              (`|ExecutionSequence`
                                                (:`then_0`
                                                  (bind _returnvalue_10 (`self.GetComponentByClass` _asadvanced_character "/Script/Mordhau.MordhauVehicleComponent"))
                                                  (`/Engine/EditorBlueprintResources/StandardMacros.IsValid` _returnvalue_10
                                                    (:`Is Valid`
                                                      (`MordhauVehicleComponent.StopDriving` _returnvalue_10))))
                                                (:`then_1`
                                                  (`AdvancedCharacter.Suicide` _asadvanced_character))))
                                            (:`CastFailed`
                                              (`self.K2_DestroyActor` _removedactor))))))))))))))
                    (:`then_1`
                      (bind _tags (`Actor.Tags` _returnvalue_8))
                      (`KismetArrayLibrary.Array_Add` _tags "pmrw")
                      (`KismetArrayLibrary.Array_Add` _tags "pmrw newobjs"))))))))))))

(fn `SetupMeshPreview`
  (bind _previewmeshcomponent (`self.PreviewMeshComponent`))
  (`/Engine/EditorBlueprintResources/StandardMacros.IsValid` _previewmeshcomponent
    (:`Is Valid`
      (`|ExecutionSequence`
        (:`then_1`
          (`SceneComponent.SetAbsolute` _previewmeshcomponent true true true)
          (`PrimitiveComponent.SetCollisionEnabled` _previewmeshcomponent "NoCollision")
          (for _index (range (`PrimitiveComponent.GetNumMaterials` _previewmeshcomponent))
            (`PrimitiveComponent.CreateDynamicMaterialInstance` _previewmeshcomponent _index "/Game/Mordhau/Assets/Materials/M_PreviewMesh.M_PreviewMesh" "None")))))))

(fn `Update Trace Text`
  (params (`Trace Placement Text` :type Text) (IgnoreLastText :type Boolean) (`Valid Placement` :type Boolean))
  (locals (`New Trace Text` :type Text))
  (set `local.New Trace Text` (select `bool` (and (`KismetTextLibrary.TextIsEmpty` `Trace Placement Text`) (not `Valid Placement`)) :`false` `Trace Placement Text` :`true` "CANNOT BUILD HERE"))
  (if (or IgnoreLastText (`KismetTextLibrary.NotEqual_TextText` (`local.New Trace Text`) (`self.LastTraceText`)))
    (`|ExecutionSequence`
      (:`then_0`
        (bind _returnvalue (`MordhauHUDWidgetComponent.GetHUDWidget` (`self.GetComponentByClass` "/Script/Mordhau.MordhauHUDWidgetComponent")))
        (if (`KismetSystemLibrary.IsValid` _returnvalue)
          (`/Game/Mordhau/UI/Ingame/BP_EquipmentWidget.UpdateEquipmentReason` (cast `/Game/Mordhau/UI/Ingame/BP_EquipmentWidget` _returnvalue :!pure true) (`KismetTextLibrary.Conv_TextToString` (`local.New Trace Text`)))))
      (:`then_1`
        (set `self.LastTraceText` (`local.New Trace Text`))))))

(fn `UpdateEquipmentUI`
  (bind _objecttype (`self.ObjectType`))
  (bind _spawnableobjects (`BuildingSystemComponent.SpawnableObjects` (`self.BuildingSystem`)))
  (bind (_preview _previewskeletal _cost _rotationoffset _rotationoffsetpreview _nothitrotationpreviewoffset _nothitlocationpreviewoffset _scalepreview _actorclass _displayname _placablelimitname _placeablelimitmax) (break `SpawnableObjectInfo` (`|GetArrayItem` _spawnableobjects _objecttype)))
  (if (`KismetArrayLibrary.Array_IsValidIndex` _spawnableobjects _objecttype)
    (bind _amount (`self.GetAmountOfPlacedEquipment` _placablelimitname))
    (bind _returnvalue (`MordhauHUDWidgetComponent.GetHUDWidget` (`self.GetComponentByClass` "/Script/Mordhau.MordhauHUDWidgetComponent")))
    (if (`KismetSystemLibrary.IsValid` _returnvalue)
      (`/Game/Mordhau/UI/Ingame/BP_EquipmentWidget.UpdateEquipmentText` (cast `/Game/Mordhau/UI/Ingame/BP_EquipmentWidget` _returnvalue :!pure true) _displayname _amount _placeablelimitmax))))

(fn `UserConstructionScript`)

(fn `ValidateDeployableSpawnConditions`
  (returns (Result :type Integer))
  (locals (FoundSpawns :type Integer) (OurTeam :type Integer))
  (bind _returnvalue (`self.GetParentCharacter`))
  (bind _returnvalue_2 (`KismetMathLibrary.Vector_One`))
  (bind _returnvalue_3 (`Pawn.GetController` _returnvalue))
  (`/Engine/EditorBlueprintResources/StandardMacros.IsValid` _returnvalue
    (:`Is Valid`
      (`/Engine/EditorBlueprintResources/StandardMacros.IsValid` _returnvalue_3
        (:`Is Valid`
          (bind _asmordhau_player_state (cast `MordhauPlayerState` (`Controller.PlayerState` _returnvalue_3))
            (:`then`
              (bind (_outactors _returnvalue_4) (`KismetSystemLibrary.BoxOverlapActors` (`self.K2_GetActorLocation` _returnvalue) (* _returnvalue_2 550.0) (`|MakeArray` "ObjectTypeQuery10" :!type "EObjectTypeQuery Enum") "/Game/Mordhau/Blueprints/GameModes/BP_SpawnProtectionBox.BP_SpawnProtectionBox_C"))
              (if _returnvalue_4
                (return 1) ; Too close to spawn
                (else
                  (bind (_outactors_2 _returnvalue_5) (`KismetSystemLibrary.BoxOverlapActors` (`self.K2_GetActorLocation`) (* _returnvalue_2 1000.0) (`|MakeArray` "ObjectTypeQuery10" :!type "EObjectTypeQuery Enum") "/Game/Mordhau/Blueprints/GameModes/Battle/BP_CapturePoint.BP_CapturePoint_C"))
                  (if _returnvalue_5
                    (return 2) ; Too close to objective
                    (else
                      (bind _asbp_frontline_game_state (cast `/Game/Mordhau/Blueprints/GameModes/Battle/BP_FrontlineGameState` (`GameplayStatics.GetGameState`))
                        (:`then`
                          (for _array_element (`/Game/Mordhau/Blueprints/GameModes/Battle/BP_FrontlineGameState.DeployableSpawns` _asbp_frontline_game_state)
                            (if (== (`self.GetOwner` _array_element) _returnvalue_3)
                              _
                              (elif (== (`/Game/Mordhau/Blueprints/Interactables/Environment/Specific/BP_DeployableSpawn.Team` _array_element) (`KismetMathLibrary.Conv_IntToByte` (`MordhauPlayerState.Team` _asmordhau_player_state)))
                                (bind _output_get (set `local.FoundSpawns` (+ (`local.FoundSpawns`) 1)))
                                (if (>= _output_get 10)
                                  (return 3) ; Too many spawns
                                  (elif (< (`self.GetDistanceTo` _array_element self) 1000.0)
                                    (return 4) ; Too close to deployable spawn
                                  ))))))
                        (:`CastFailed`
                          _)))))))
            (:`CastFailed`
              _)))
        (:`Is Not Valid`
          _)))
    (:`Is Not Valid`
      _))
  (return 0))

(fn `ValidateSpotWithBuildingSystem`
  (params (Offset :type "Vector Structure") (DisplayObjectPreview :type Boolean))
  (returns (Succeeded :type Boolean) (Location :type "Vector Structure") (Rotation :type "Rotator Structure") (AttachToComponent :type "SceneComponent Object Reference"))
  (`|ExecutionSequence`
    (:`then_0`
      (if (== (`.ActorClass` (break `SpawnableObjectInfo` (`|GetArrayItem` (`BuildingSystemComponent.SpawnableObjects` (`self.BuildingSystem`)) (`self.ObjectType`)))) "/Game/Mordhau/Blueprints/Interactables/Environment/Specific/BP_DeployableSpawn.BP_DeployableSpawn_C")
        (bind _result (`self.ValidateDeployableSpawnConditions`))
        (if (!= _result 0)
          (bind (_outlocation _outrotation _attachtocomponent _buildabletracehit _returnvalue) (`BuildingSystemComponent.ValidateSpot` (`self.BuildingSystem`) Offset (`self.ObjectType`) DisplayObjectPreview true))
          (`|ExecutionSequence`
            (:`then_0`
              (switch `int` _result
                (:`1`
                  (`self.Update Trace Text` "TOO CLOSE TO SPAWN AREA"))
                (:`2`
                  (`self.Update Trace Text` "TOO CLOSE TO OBJECTIVE"))
                (:`3`
                  (`self.Update Trace Text` "TEAM HAS TOO MANY SPAWNS"))
                (:`4`
                  (`self.Update Trace Text` "TOO CLOSE TO EXISTING SPAWN"))))
            (:`then_1`
              (return _returnvalue _outlocation _outrotation _attachtocomponent))))))
    (:`then_1`
      (bind (_outlocation_2 _outrotation_2 _attachtocomponent_2 _buildabletracehit_2 _returnvalue_2) (`BuildingSystemComponent.ValidateSpot` (`self.BuildingSystem`) Offset (`self.ObjectType`) DisplayObjectPreview false))
      (if (`KismetSystemLibrary.IsValid` _buildabletracehit_2)
        (`self.Update Trace Text` (`BuildableTraceBase.TraceTextForUI` _buildabletracehit_2) false _returnvalue_2)
        (else
          (`self.Update Trace Text` "" false _returnvalue_2)))
      (return _returnvalue_2 _outlocation_2 _outrotation_2 _attachtocomponent_2))))